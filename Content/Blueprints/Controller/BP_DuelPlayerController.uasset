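; Player controller for a sheriff-versus-gunman duel that stages the cinematic outcome of each duel event.
; BeginPlay binds Hit, Dodge, Fire, FireComplete and FightBack delegates, whose handlers use timed delays to drive level sequences, camera switches, montages and temporary bullets.
; Handlers update DuelGameState and its duelists: Dodge resets the round, while firing handlers mark the victim dead.
; Hit, FireComplete and FightBack end with an authority-only return-to-lobby widget.
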(event Custom|DodgeDelegate_이벤트
  (bind _outactors (Actor|GetAllActorsOfClass "/Script/Engine.CameraActor"))
  (Game|Player|SetViewTargetwithBlend (Utilities|Array|Get(acopy) _outactors 1) 0.0 "VTBlend_Linear" 0.0 false)
  (Utilities|FlowControl|Delay 2.5)
  (Game|Player|SetViewTargetwithBlend (Utilities|Array|Get(acopy) _outactors) 0.0 "VTBlend_Linear" 0.0 false)
  (bind _asduel_game_state (Utilities|Casting|CastToDuelGameState (Game|GetGameState)))
  (Class|DuelGameState|ResetDuelState _asduel_game_state)
  (if (not (Variables|/Script/WildWest.DuelGameState|GetbIsDuelOver _asduel_game_state))
    (Default|CallSetWidgetVisible)))

(event Custom|FireDelegate_이벤트
  (Utilities|FlowControl|Delay 0.3)
  (bind _asduel_game_state (Utilities|Casting|CastToDuelGameState (Game|GetGameState)))
  (switch Utilities|FlowControl|Switch|SwitchonEDuelState (Variables|/Script/WildWest.DuelGameState|GetSheriffDuelState _asduel_game_state)
    (:EDS_Left
      (Variables|Default|SetSpawnTransform (Math|Transform|MakeTransform (.location (Variables|Default|GetSpawnTransform)) "1.200000,185.000000,0.000000" "1.000000,1.000000,1.000000")))
    (:EDS_Middle
      _)
    (:EDS_Right
      (Variables|Default|SetSpawnTransform (Math|Transform|MakeTransform (.location (Variables|Default|GetSpawnTransform)) "1.200000,175.000000,0.000000" "1.000000,1.000000,1.000000"))))
  (bind _returnvalue (Game|SpawnActorfromClass "/Game/Blueprints/Gun/BP_Bullet.BP_Bullet_C" (Variables|Default|GetSpawnTransform) "Undefined" 0 0))
  (Utilities|FlowControl|Delay 3.79)
  (Actor|DestroyActor _returnvalue)
  (bind _asduel_game_state_2 (Utilities|Casting|CastToDuelGameState (Game|GetGameState)))
  (Class|DuelGameState|ResetDuelState _asduel_game_state_2)
  (Class|DuelSheriff|SetIsDead (Variables|/Script/WildWest.DuelGameState|GetDuelSheriff _asduel_game_state_2) true))

(event Custom|FireCompleteDelegate_이벤트
  (Utilities|FlowControl|Delay 2.5)
  (bind _asduel_game_state (Utilities|Casting|CastToDuelGameState (Game|GetGameState)))
  (Class|DuelSheriff|SetIsSlow (Variables|/Script/WildWest.DuelGameState|GetDuelSheriff _asduel_game_state) true)
  (Class|DuelSheriff|SetShoot (Variables|/Script/WildWest.DuelGameState|GetDuelSheriff _asduel_game_state) true)
  (bind _returnvalue (Sequencer|Player|CreateLevelSequencePlayer "/Game/Cutscene/FinalMasterSequence.FinalMasterSequence"))
  (Sequencer|Player|Play _returnvalue :!class /Script/MovieScene.MovieSceneSequencePlayer)
  (Utilities|FlowControl|Delay 3.0)
  (bind _asduel_game_state_2 (Utilities|Casting|CastToDuelGameState (Game|GetGameState)))
  (Animation|PlayAnimMontage (Variables|/Script/WildWest.DuelGameState|GetDuelSheriff _asduel_game_state_2) "/Game/PolygonWestern/Animations/Sheriff/Sheriff_ShootRevolver_Montage.Sheriff_ShootRevolver_Montage" 0.4 "None")
  (Utilities|FlowControl|Delay 0.3)
  (bind _returnvalue_2 (Game|SpawnActorfromClass "/Game/Blueprints/Gun/BP_Bullet.BP_Bullet_C" (Math|Transform|MakeTransform "-580.000000,0.000000,140.000000" "1.200000,0.000000,0.000000" "1.000000,1.000000,1.000000") "Undefined" 0 0))
  (Utilities|FlowControl|Delay 3.79)
  (Actor|DestroyActor _returnvalue_2)
  (bind _asduel_game_state_3 (Utilities|Casting|CastToDuelGameState (Game|GetGameState)))
  (Class|DuelGunman|SetIsDead (Variables|/Script/WildWest.DuelGameState|GetDuelGunman _asduel_game_state_3) true)
  (Utilities|FlowControl|Delay 2.91)
  (bind _returnvalue_3 (Actor|GetActorOfClass "/Script/Engine.CameraActor"))
  (Game|Player|SetViewTargetwithBlend _returnvalue_3 0.0 "VTBlend_Linear" 0.0 false)
  (if (Ability|HasAuthority)
    (bind _returnvalue_4 (UserInterface|CreateWidget "/Game/Blueprints/HUD/WBP_ReturnToLobby.WBP_ReturnToLobby_C"))
    (Class|ReturntoLobby|ReturntoLobbySetup _returnvalue_4)))

(event Custom|HitDelegate_이벤트
  (bind _returnvalue (Sequencer|Player|CreateLevelSequencePlayer "/Game/Cutscene/MasterSequence.MasterSequence"))
  (Sequencer|Player|Play _returnvalue :!class /Script/MovieScene.MovieSceneSequencePlayer)
  (bind _returnvalue_2 (Actor|GetActorOfClass "/Script/Engine.CameraActor"))
  (Utilities|FlowControl|Delay 7.0)
  (Game|Player|SetViewTargetwithBlend _returnvalue_2 0.0 "VTBlend_Linear" 0.0 false)
  (if (Ability|HasAuthority)
    (bind _returnvalue_3 (UserInterface|CreateWidget "/Game/Blueprints/HUD/WBP_ReturnToLobby.WBP_ReturnToLobby_C"))
    (Class|ReturntoLobby|ReturntoLobbySetup _returnvalue_3)))

(event Custom|FightBackDelegate_이벤트
  (Utilities|FlowControl|Delay 2.5)
  (bind _returnvalue (Sequencer|Player|CreateLevelSequencePlayer "/Game/Cutscene/FightBackMasterSequence.FightBackMasterSequence"))
  (Sequencer|Player|Play _returnvalue :!class /Script/MovieScene.MovieSceneSequencePlayer)
  (bind _asduel_game_state (Utilities|Casting|CastToDuelGameState (Game|GetGameState)))
  (Animation|PlayAnimMontage (Variables|/Script/WildWest.DuelGameState|GetDuelSheriff _asduel_game_state) "/Game/PolygonWestern/Animations/Sheriff/Sheriff_ShootRevolver_Montage.Sheriff_ShootRevolver_Montage" 0.25 "None")
  (Utilities|FlowControl|Delay 0.3)
  (bind _returnvalue_2 (Game|SpawnActorfromClass "/Game/Blueprints/Gun/BP_Bullet.BP_Bullet_C" (Math|Transform|MakeTransform "-580.000000,0.000000,140.000000" "1.200000,0.000000,0.000000" "1.000000,1.000000,1.000000") "Undefined" 0 0))
  (Utilities|FlowControl|Delay 3.79)
  (Actor|DestroyActor _returnvalue_2)
  (bind _asduel_game_state_2 (Utilities|Casting|CastToDuelGameState (Game|GetGameState)))
  (Class|DuelGunman|SetIsDead (Variables|/Script/WildWest.DuelGameState|GetDuelGunman _asduel_game_state_2) true)
  (Utilities|FlowControl|Delay 2.91)
  (bind _returnvalue_3 (Actor|GetActorOfClass "/Script/Engine.CameraActor"))
  (Game|Player|SetViewTargetwithBlend _returnvalue_3 0.0 "VTBlend_Linear" 0.0 false)
  (if (Ability|HasAuthority)
    (bind _returnvalue_4 (UserInterface|CreateWidget "/Game/Blueprints/HUD/WBP_ReturnToLobby.WBP_ReturnToLobby_C"))
    (Class|ReturntoLobby|ReturntoLobbySetup _returnvalue_4)))

(event EventBeginPlay
  (EventDispatchers|AssignHitDelegate (delegate Custom|HitDelegate_이벤트))
  (EventDispatchers|AssignDodgeDelegate (delegate Custom|DodgeDelegate_이벤트))
  (EventDispatchers|AssignFireDelegate (delegate Custom|FireDelegate_이벤트))
  (EventDispatchers|AssignFireCompleteDelegate (delegate Custom|FireCompleteDelegate_이벤트))
  (EventDispatchers|AssignFightBackDelegate (delegate Custom|FightBackDelegate_이벤트)))

(fn ConstructionScript)