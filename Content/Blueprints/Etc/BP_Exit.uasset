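; BP_Exit is an exit trigger that awards victory to a Gunman who reaches it after opening all vaults.
; On authority, its Collision overlap compares the Gunman's VaultOpened count with the vault total held by BP_TownGameMode.
; On a match, it calls the Gunman victory creation on the game mode's server player controller, then the client variant on its client player controller.
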(event OnComponentBeginOverlap(Collision)
  (params (OverlappedComponent :type Primitive%20Component%20Object%20Reference) (OtherActor :type Actor%20Object%20Reference) (OtherComp :type Primitive%20Component%20Object%20Reference) (OtherBodyIndex :type Integer) (bFromSweep :type Boolean) (SweepResult :type Hit%20Result%20Structure%20%28by%20ref%29))
  (Networking|SwitchHasAuthority
    (:Authority
      (bind _asgunman (Utilities|Casting|CastToGunman OtherActor))
      (bind _asbp_town_game_mode (Utilities|Casting|CastToBP_TownGameMode (Game|GetGameMode)))
      (if (== (Variables|/Game/Blueprints/GameModes/BP_TownGameMode.BP_TownGameMode_C|GetNumberOfVault _asbp_town_game_mode) (Variables|/Script/WildWest.Gunman|GetVaultOpened _asgunman))
        (bind _asbp_town_player_controller (Utilities|Casting|CastToBP_TownPlayerController (Variables|/Game/Blueprints/GameModes/BP_TownGameMode.BP_TownGameMode_C|GetServerPlayerController _asbp_town_game_mode)))
        (Default|CreateGunmanVictory _asbp_town_player_controller)
        (bind _asbp_town_player_controller_2 (Utilities|Casting|CastToBP_TownPlayerController (Variables|/Game/Blueprints/GameModes/BP_TownGameMode.BP_TownGameMode_C|GetClientPlayerController _asbp_town_game_mode)))
        (Default|ClientCreateGunmanVictory _asbp_town_player_controller_2)))))

(fn ConstructionScript)