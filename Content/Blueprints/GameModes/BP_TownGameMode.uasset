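; Town game mode that spawns and possesses a Gunman or Sheriff pawn for the first two players to log in.
; The game instance's server or client character state picks each role.
; A host Sheriff also creates local players after a short delay, spawning a Sheriff at every PlayerStart using its tag as controller ID; a client Sheriff gets a ClientCreatePlayer call instead.
; Sheriffs spawned here register in TownGameState's SheriffList.
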(event EventPostLogin
  (params (NewPlayer :type Player%20Controller%20Object%20Reference))
  (Utilities|FlowControl|DoN 2
    (:Exit
      (bind _aswild_west_game_instance (Utilities|Casting|CastToWildWestGameInstance (Game|GetGameInstance)))
      (if (== (Game|GetPlayerController 0) NewPlayer)
        (switch Utilities|FlowControl|Switch|SwitchonECharacterState (Variables|/Script/WildWest.WildWestGameInstance|GetServerCharacterState _aswild_west_game_instance)
          (:ECS_Gunman
            (bind _returnvalue (Game|SpawnActorfromClass "/Game/Blueprints/Character/BP_Gunman.BP_Gunman_C" (Variables|Default|GetGunmanTransform) "Undefined" 0 0 :!label _label))
            (Pawn|Possess NewPlayer _returnvalue))
          (:ECS_Sheriff
            (bind _returnvalue_2 (Game|SpawnActorfromClass "/Game/Blueprints/Character/BP_Sheriff.BP_Sheriff_C" (Variables|Default|GetSheriffTransform) "Undefined" 0 0 :!label _label_2))
            (Pawn|Possess NewPlayer _returnvalue_2)
            (bind _astown_game_state (Utilities|Casting|CastToTownGameState (Game|GetGameState)))
            (Utilities|Array|AddUnique (Variables|/Script/WildWest.TownGameState|GetSheriffList _astown_game_state) _returnvalue_2)
            (bind _asbp_town_player_controller (Utilities|Casting|CastToBP_TownPlayerController NewPlayer))
            (if (== NewPlayer (Game|GetPlayerController 0))
              (Utilities|FlowControl|Delay 1.0)
              (bind _outactors (Actor|GetAllActorsOfClass "/Script/Engine.PlayerStart"))
              (for _array_element _outactors
                (bind _returnvalue_3 (Class|GameplayStatics|CreatePlayer (CallFunction|TagtoInt _array_element)))
                (bind _returnvalue_4 (Game|SpawnActorfromClass "/Game/Blueprints/Character/BP_Sheriff.BP_Sheriff_C" (Transformation|GetActorTransform _array_element) "Undefined" 0 0))
                (Pawn|Possess _returnvalue_3 _returnvalue_4)
                (bind _astown_game_state_2 (Utilities|Casting|CastToTownGameState (Game|GetGameState)))
                (Utilities|Array|AddUnique (Variables|/Script/WildWest.TownGameState|GetSheriffList _astown_game_state_2) _returnvalue_4))
              (else
                (Default|ClientCreatePlayer _asbp_town_player_controller)))))
        (else
          (switch Utilities|FlowControl|Switch|SwitchonECharacterState (Variables|/Script/WildWest.WildWestGameInstance|GetClientCharacterState _aswild_west_game_instance)
            (:ECS_Gunman
              (goto _label))
            (:ECS_Sheriff
              (goto _label_2))))))))

(fn ConstructionScript)

(fn TagtoInt
  (params (PlayerStart :type Player%20Start%20Object%20Reference))
  (return (Math|Conversions|ToInteger(Byte) (Utilities|String|ToString(Name) (Variables|/Script/Engine.PlayerStart|GetPlayerStartTag PlayerStart)))))