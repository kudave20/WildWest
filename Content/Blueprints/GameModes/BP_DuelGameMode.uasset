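; Duel game mode that sets up the server and client players as Gunman or Sheriff when they join.
; HandleStartingNewPlayer treats the local controller as server, others as client, storing one of each in DuelGameState via DoOnce.
; Each side's role from WildWestGameInstance selects the pawn to spawn at a fixed transform and possess.
; Both roles view through the level's CameraActor; only the Gunman also gets an initial control rotation.
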(event EventHandleStartingNewPlayer
  (params (NewPlayer :type Player%20Controller%20Object%20Reference))
  (bind _aswild_west_game_instance (Utilities|Casting|CastToWildWestGameInstance (Game|GetGameInstance)))
  (bind _asduel_game_state (Utilities|Casting|CastToDuelGameState (Game|GetGameState)))
  (bind _asduel_player_controller (Utilities|Casting|CastToDuelPlayerController NewPlayer))
  (if (Pawn|IsLocalPlayerController NewPlayer)
    (Utilities|FlowControl|DoOnce false
      (:Completed
        (Variables|/Script/WildWest.DuelGameState|SetServerPlayerController _asduel_game_state _asduel_player_controller)
        (switch Utilities|FlowControl|Switch|SwitchonECharacterState (Variables|/Script/WildWest.WildWestGameInstance|GetServerCharacterState _aswild_west_game_instance)
          (:ECS_Gunman
            (bind _returnvalue (Game|SpawnActorfromClass "/Game/Blueprints/Character/BP_DuelGunman.BP_DuelGunman_C" (Math|Transform|MakeTransform "0.000000,0.000000,88.000000" "0.000000,-90.000000,0.000000" "1.000000,1.000000,1.000000") "Undefined" 0 0 :!label _label))
            (Pawn|Possess NewPlayer _returnvalue)
            (bind _asduel_player_controller_2 (Utilities|Casting|CastToDuelPlayerController NewPlayer))
            (Class|DuelPlayerController|SetInitialControlRotation _asduel_player_controller_2 (Math|Rotator|MakeRotator 0.0 0.0 -9e+01)))
          (:ECS_Sheriff
            (bind _returnvalue_2 (Game|SpawnActorfromClass "/Game/Blueprints/Character/BP_DuelSheriff.BP_DuelSheriff_C" (Math|Transform|MakeTransform "-700.000000,0.000000,88.000000" "0, 0, 0" "1.000000,1.000000,1.000000") "Undefined" 0 0 :!label _label_2))
            (Pawn|Possess NewPlayer _returnvalue_2)))))
    (else
      (Utilities|FlowControl|DoOnce false
        (:Completed
          (Variables|/Script/WildWest.DuelGameState|SetClientPlayerController _asduel_game_state _asduel_player_controller)
          (switch Utilities|FlowControl|Switch|SwitchonECharacterState (Variables|/Script/WildWest.WildWestGameInstance|GetClientCharacterState _aswild_west_game_instance)
            (:ECS_Gunman
              (goto _label))
            (:ECS_Sheriff
              (goto _label_2)))))))
  (bind _returnvalue_3 (Actor|GetActorOfClass "/Script/Engine.CameraActor"))
  (Game|Player|SetViewTargetwithBlend NewPlayer _returnvalue_3 0.0 "VTBlend_Linear" 0.0 false))

(fn ConstructionScript)