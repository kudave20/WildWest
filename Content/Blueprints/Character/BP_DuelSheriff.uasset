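; BP_DuelSheriff is a character Blueprint for the sheriff in a duel, whose event graph currently does nothing.
; Its possession, client widget, selection-complete and visibility events are all empty, and the construction script is empty too.
; Disconnected leftover logic would create duel and dodge widgets, bind controller delegates, toggle those widgets with UI-only input, and start the GameState duel timer on the server.
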(event Custom|DuelSelectCompleteDelegate_이벤트)

(event Custom|SetWidgetVisible_이벤트)

(event Custom|ClientCreateWidget)

(event EventPossessed
  (params (NewController :type Controller%20Object%20Reference)))

(fn ConstructionScript)